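; BP_ShapeShifter is the player's shape-shifter, morphed through a material parameter to match incoming wall shapes.
; Two held inputs raise or lower ShapeShiftValue on a dynamic material instance each tick, clamped 0 to 1, and cancel when both are held.
; CalculateOutcome compares that value to the wall's within a tolerance.
; A match adds score and combo in BP_GameState, while a miss resets combo with a stronger camera shake.
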(event Custom|CalculateOutcome
  (params (WallShapeValue :type Float%20%28single-precision%29))
  (bind _gamestateref (Variables|Default|GetGameStateRef))
  ;[0.001582 0.000696 0.005208] Calculate outcome with walls collided
  (bind _returnvalue (Rendering|Material|GetScalarParameterValue (Variables|Default|GetPlayerMat) "ShapeShiftValue" :!class /Script/Engine.MaterialInstanceDynamic))
  (if (Math|Float|NearlyEqual(Float) WallShapeValue _returnvalue (Variables|Default|GetShapeDifference))
    (Default|AddScore _gamestateref 0.0 1)
    (Default|AddCombo _gamestateref)
    (Class|PlayerController|ClientPlayCameraShake (Game|GetPlayerController 0) "/Game/Khizer/Blueprint/CameraShake/BP_CameraShake.BP_CameraShake_C" 1.0 "CameraLocal" "4.000000, 0,3.000000")
    (else
      (Default|ResetCombo (Variables|Default|GetGameStateRef))
      (Class|PlayerController|ClientPlayCameraShake (Game|GetPlayerController 0) "/Game/Khizer/Blueprint/CameraShake/BP_CameraShake.BP_CameraShake_C" 3.0 "CameraLocal" "4.000000, 0,3.000000"))))

(event EventBeginPlay
  (Utilities|FlowControl|Sequence
    (:then_0
      (bind _returnvalue (Rendering|Material|CreateDynamicMaterialInstance (Variables|Default|GetPlayer) 0 0 :!class /Script/Engine.PrimitiveComponent))
      (Variables|Default|SetPlayerMat _returnvalue)
      (bind _asbp_game_state (Utilities|Casting|CastToBP_GameState (Game|GetGameState)))
      (Variables|Default|SetGameStateRef _asbp_game_state))))

(event EventTick
  (params (DeltaSeconds :type Float%20%28single-precision%29))
  (bind _returnvalue (Utilities|Time|GetWorldDeltaSeconds))
  (bind _brightmousedown (Variables|Default|GetbRightMouseDown))
  (bind _shapeshiftspeed (Variables|Default|GetShapeShiftSpeed))
  (bind _returnvalue_2 (* _shapeshiftspeed _returnvalue))
  ;[0 0 0] Check if only 1 Button is pressed
  (if (Variables|Default|GetbLeftMouseDown)
    (if (not _brightmousedown)
      (bind _returnvalue_3 (Rendering|Material|GetScalarParameterValue (Variables|Default|GetPlayerMat) "ShapeShiftValue" :!class /Script/Engine.MaterialInstanceDynamic))
      (Rendering|Material|SetScalarParameterValue (Variables|Default|GetPlayerMat) "ShapeShiftValue" (Math|Float|Clamp(Float) (+ _returnvalue_3 _returnvalue_2)) :!class /Script/Engine.MaterialInstanceDynamic))
    (elif _brightmousedown
      (bind _returnvalue_4 (Rendering|Material|GetScalarParameterValue (Variables|Default|GetPlayerMat) "ShapeShiftValue" :!class /Script/Engine.MaterialInstanceDynamic))
      (Rendering|Material|SetScalarParameterValue (Variables|Default|GetPlayerMat) "ShapeShiftValue" (Math|Float|Clamp(Float) (- _returnvalue_4 _returnvalue_2)) :!class /Script/Engine.MaterialInstanceDynamic))))

(event Input|ActionEvents|InputActionShapeShiftNext
  (params (Key :type Key%20Structure))
  (:Pressed
    (Variables|Default|SetbLeftMouseDown true))
  (:Released
    (Variables|Default|SetbLeftMouseDown false)))

(event Input|ActionEvents|InputActionShapeShiftPrevious
  (params (Key :type Key%20Structure))
  (:Pressed
    (Variables|Default|SetbRightMouseDown true))
  (:Released
    (Variables|Default|SetbRightMouseDown false)))

(fn ConstructionScript)