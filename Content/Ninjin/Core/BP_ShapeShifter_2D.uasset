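; Shape-matching game prototype where the player steers a 2D shape value to match a randomly generated wall shape before each round ends.
; Tick adds input axes, clamps the result and feeds it to the player Substance graph's "Location" input, rendering synchronously every frame.
; A looping timeline tints the wall, then on finish prints hit or miss from the summed axis difference against a threshold and re-randomizes the wall's Substance shape.
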(event EventBeginPlay
  (bind _currentplayershape (Variables|Default|GetCurrentPlayerShape))
  (bind _currentwallshape (Variables|Default|GetCurrentWallShape))
  (bind _returnvalue (- _currentwallshape _currentplayershape))
  (bind _returnvalue_2 (Rendering|Material|CreateDynamicMaterialInstance (Variables|Default|GetWall) 0 0 :!class /Script/Engine.PrimitiveComponent))
  (Variables|Default|SetWallColorDMI _returnvalue_2)
  (CallFunction|CreateNewWallShape)
  (bind _wallcolor (Timeline|GameLoopInTimelineLInPawnLMAO PlayFromStart)
    (:Update
      (Rendering|Material|SetVectorParameterValueonMaterials (Variables|Default|GetWall) "Color" (Math|Conversions|ToVector(LinearColor) _wallcolor)))
    (:Finished
      (Utilities|FlowControl|Sequence
        (:then_0
          (if (< (+ (Math|Float|Absolute(Float) (.x _returnvalue)) (Math|Float|Absolute(Float) (.y _returnvalue))) (Variables|Default|GetShapeDifference))
            (Development|PrintString (Variables|Default|GetHitString) true true "(R=0.000000,G=1.000000,B=0.000000,A=1.000000)" 3.0)
            (else
              (Development|PrintString (Variables|Default|GetMissString) true true "(R=1.000000,G=0.000000,B=0.000000,A=1.000000)" 3.0))))
        (:then_1
          (CallFunction|CreateNewWallShape)
          (Timeline|GameLoopInTimelineLInPawnLMAO PlayFromStart))))))

(event EventTick
  (params (DeltaSeconds :type Float%20%28single-precision%29))
  (bind _substance_player (Variables|Default|GetSubstance_Player))
  (bind _mouseyspeed (Variables|Default|GetMouseYSpeed))
  (bind _returnvalue (* DeltaSeconds _mouseyspeed))
  (bind _output_get (Variables|Default|SetCurrentPlayerShape (Math|Vector2D|MakeVector2D (Math|Float|Clamp(Float) (.x (+ (Variables|Default|GetCurrentPlayerShape) (Math|Vector2D|MakeVector2D (* _returnvalue (Class|Actor|GetInputAxisKeyValue)) (* (Class|Actor|GetInputAxisKeyValue) _returnvalue 1.777778)))) -1.0) (Math|Float|Clamp(Float) (.y (+ (Variables|Default|GetCurrentPlayerShape) (Math|Vector2D|MakeVector2D (* _returnvalue (Class|Actor|GetInputAxisKeyValue)) (* (Class|Actor|GetInputAxisKeyValue) _returnvalue 1.777778)))) -1.0))))
  (Class|SubstanceGraphInstance|SetInputFloat _substance_player "Location" (Utilities|Array|MakeArray (.x _output_get) (.y _output_get)))
  (Class|SubstanceUtility|SyncRendering _substance_player))

(fn ConstructionScript)

(fn CreateNewWallShape
  (bind _substance_wall (Variables|Default|GetSubstance_Wall))
  (bind _output_get (Variables|Default|SetCurrentWallShape (Math|Vector2D|MakeVector2D (Math|Random|RandomFloatinRange -1.0 1.0) (Math|Random|RandomFloatinRange -1.0 1.0))))
  (Class|SubstanceGraphInstance|SetInputFloat _substance_wall "Location" (Utilities|Array|MakeArray (.x _output_get) (.y _output_get)))
  (Class|SubstanceUtility|SyncRendering _substance_wall))