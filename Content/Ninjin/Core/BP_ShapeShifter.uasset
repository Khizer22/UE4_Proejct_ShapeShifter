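; BP_ShapeShifter is a shape-matching minigame actor where a player mesh morphs to fit a repeatedly approaching wall.
; Dynamic materials on Player and Wall share a ShapeShiftValue parameter, which holding left or right mouse raises or lowers on the player each Tick.
; A looping WallSpawner timeline moves the wall along X, then prints hit or miss by comparing both values within ShapeDifference and re-randomizes the wall.
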(event EventBeginPlay
  (Utilities|FlowControl|Sequence
    (:then_0
      (bind _returnvalue (Rendering|Material|CreateDynamicMaterialInstance (Variables|Default|GetPlayer) 0 0 :!class /Script/Engine.PrimitiveComponent))
      (Variables|Default|SetPlayerMat _returnvalue)
      (bind _returnvalue_2 (Rendering|Material|CreateDynamicMaterialInstance (Variables|Default|GetWall) 0 0 :!class /Script/Engine.PrimitiveComponent))
      (Variables|Default|SetWallMat _returnvalue_2))
    (:then_1
      (Rendering|Material|SetScalarParameterValue (Variables|Default|GetWallMat) "ShapeShiftValue" (Math|Random|RandomFloat) :!class /Script/Engine.MaterialInstanceDynamic)
      (bind _distancefromplayer (Timeline|WallSpawner PlayFromStart)
        (:Update
          (Transformation|SetRelativeLocation (Variables|Default|GetWall) (Math|Vector|MakeVector _distancefromplayer 0.0 0.0) false true))
        (:Finished
          (Utilities|FlowControl|Sequence
            (:then_0
              (bind _returnvalue_3 (Rendering|Material|GetScalarParameterValue (Variables|Default|GetPlayerMat) "ShapeShiftValue" :!class /Script/Engine.MaterialInstanceDynamic))
              (bind _returnvalue_4 (Rendering|Material|GetScalarParameterValue (Variables|Default|GetWallMat) "ShapeShiftValue" :!class /Script/Engine.MaterialInstanceDynamic))
              (Development|PrintString (Utilities|String|SelectString (Variables|Default|GetHitString) (Variables|Default|GetMissString) (Math|Float|NearlyEqual(Float) _returnvalue_4 _returnvalue_3 (Variables|Default|GetShapeDifference))) true true "(R=1.000000,G=0.630607,B=0.000000,A=1.000000)"))
            (:then_1
              (Rendering|Material|SetScalarParameterValue (Variables|Default|GetWallMat) "ShapeShiftValue" (Math|Random|RandomFloat) :!class /Script/Engine.MaterialInstanceDynamic)
              (Timeline|WallSpawner PlayFromStart))))))))

(event EventTick
  (params (DeltaSeconds :type Float%20%28single-precision%29))
  (bind _returnvalue (Utilities|Time|GetWorldDeltaSeconds))
  (bind _brightmousedown (Variables|Default|GetbRightMouseDown))
  (bind _shapeshiftspeed (Variables|Default|GetShapeShiftSpeed))
  (bind _returnvalue_2 (* _shapeshiftspeed _returnvalue))
  ;[0 0 0] Check if only 1 Button is pressed
  (if (Variables|Default|GetbLeftMouseDown)
    (if (not _brightmousedown)
      (bind _returnvalue_3 (Rendering|Material|GetScalarParameterValue (Variables|Default|GetPlayerMat) "ShapeShiftValue" :!class /Script/Engine.MaterialInstanceDynamic))
      (Rendering|Material|SetScalarParameterValue (Variables|Default|GetPlayerMat) "ShapeShiftValue" (Math|Float|Clamp(Float) (+ _returnvalue_3 _returnvalue_2)) :!class /Script/Engine.MaterialInstanceDynamic))
    (elif _brightmousedown
      (bind _returnvalue_4 (Rendering|Material|GetScalarParameterValue (Variables|Default|GetPlayerMat) "ShapeShiftValue" :!class /Script/Engine.MaterialInstanceDynamic))
      (Rendering|Material|SetScalarParameterValue (Variables|Default|GetPlayerMat) "ShapeShiftValue" (Math|Float|Clamp(Float) (- _returnvalue_4 _returnvalue_2)) :!class /Script/Engine.MaterialInstanceDynamic))))

(event Input|MouseEvents|LeftMouseButton
  (params (Key :type Key%20Structure))
  (:Pressed
    (Variables|Default|SetbLeftMouseDown true))
  (:Released
    (Variables|Default|SetbLeftMouseDown false)))

(event Input|MouseEvents|RightMouseButton
  (params (Key :type Key%20Structure))
  (:Pressed
    (Variables|Default|SetbRightMouseDown true))
  (:Released
    (Variables|Default|SetbRightMouseDown false)))

(fn ConstructionScript)