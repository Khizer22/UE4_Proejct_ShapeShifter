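; BP_ShifterRocksmith is a player shape-shifter that morphs to match incoming wall shapes for score and combo.
; Tick integrates move-axis input into a clamped 2D shape value, shows it as debug text, and feeds it to a Substance rendered asynchronously.
; CalculateOutcome compares the wall's shape to the player's by vector distance, adding score and combo within tolerance or resetting combo, with a camera shake either way.
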(event Custom|CalculateOutcome
  (params (WallShapeValue :type Vector%202D%20Structure))
  (bind _gamestateref (Variables|Default|GetGameStateRef))
  ;[0 0 0] Calculate outcome with walls collided
  (bind _output_get (Variables|Default|SetShapeDifferenceCurrent (Math|Vector2D|Vector2DLength (- WallShapeValue (Variables|Default|GetCurrentPlayerShape)))))
  (if (< _output_get (Variables|Default|GetShapeDifferenceComboTolerance))
    (Default|AddScore _gamestateref (- 3.0 (Variables|Default|GetShapeDifferenceCurrent)))
    (Default|AddCombo _gamestateref)
    (Class|PlayerController|ClientPlayCameraShake (Game|GetPlayerController 0) "/Game/Khizer/Blueprint/CameraShake/BP_CameraShake.BP_CameraShake_C" 1.0 "CameraLocal" "4.000000, 0,3.000000")
    (else
      (Default|ResetCombo (Variables|Default|GetGameStateRef))
      (Class|PlayerController|ClientPlayCameraShake (Game|GetPlayerController 0) "/Game/Khizer/Blueprint/CameraShake/BP_CameraShake.BP_CameraShake_C" 3.0 "CameraLocal" "4.000000, 0,3.000000"))))

(event EventBeginPlay
  (bind _asbp_game_state (Utilities|Casting|CastToBP_GameState (Game|GetGameState)))
  (Variables|Default|SetGameStateRef _asbp_game_state))

(event EventTick
  (params (DeltaSeconds :type Float%20%28single-precision%29))
  (bind _substance (Variables|Default|GetSubstance))
  (Utilities|FlowControl|Sequence
    (:then_0
      ;[0 0 0] WASD Control
      (Variables|Default|SetCurrentPlayerShape (Math|Vector2D|MakeVector2D (Math|Float|Clamp(Float) (+ (* (Utilities|Time|GetWorldDeltaSeconds) (Variables|Default|GetShapeShiftSpeed) (Input|AxisValues|GetMoveRight)) (.x (Variables|Default|GetCurrentPlayerShape)))) (Math|Float|Clamp(Float) (+ (.y (Variables|Default|GetCurrentPlayerShape)) (* (Utilities|Time|GetWorldDeltaSeconds) (Variables|Default|GetShapeShiftSpeed) (Input|AxisValues|GetMoveForward))))))
      ;[1 1 1] DEBUG
      (Rendering|Debug|DrawDebugString (Transformation|GetActorLocation) (Utilities|String|Append "My Shape: " (Utilities|String|ToString(Vector2d) (Variables|Default|GetCurrentPlayerShape))) 0 "(R=0.000000,G=0.000000,B=0.000000,A=1.000000)"))
    (:then_1
      ;[0 0 0] Update Substance
      (Class|SubstanceGraphInstance|SetInputFloat _substance "Location" (Utilities|Array|MakeArray (.x (Variables|Default|GetCurrentPlayerShape)) (.y (Variables|Default|GetCurrentPlayerShape))))
      (Class|SubstanceUtility|AsyncRendering _substance))))

(fn ConstructionScript)