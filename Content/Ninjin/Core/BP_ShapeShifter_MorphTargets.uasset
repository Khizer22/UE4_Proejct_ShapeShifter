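; Shape-shifting wall game prototype where input axes morph the player's shape as a wall repeatedly moves along X.
; Tick accumulates input into CurrentMorph, wraps it modulo 1, and maps it through a triangle wave onto the Location and Rotation morph targets.
; When the WallSpawner timeline finishes, it prints hit or miss by comparing the morph's distance from zero to ShapeDifference, randomizes the morph and restarts.
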(event EventBeginPlay
  (bind _currentmorph (Variables|Default|GetCurrentMorph))
  (CallFunction|SetCurrentOffset)
  (bind _distancefromplayer (Timeline|WallSpawner PlayFromStart)
    (:Update
      (Transformation|SetRelativeLocation (Variables|Default|GetWall) (Math|Vector|MakeVector _distancefromplayer 0.0 0.0) false true))
    (:Finished
      (Utilities|FlowControl|Sequence
        (:then_0
          (Development|PrintString (Utilities|String|SelectString (Variables|Default|GetHitString) (Variables|Default|GetMissString) (< (+ (Math|Float|Absolute(Float) (.x _currentmorph)) (Math|Float|Absolute(Float) (.y _currentmorph))) (Variables|Default|GetShapeDifference))) true true "(R=1.000000,G=0.630607,B=0.000000,A=1.000000)" 3.0))
        (:then_1
          (CallFunction|SetCurrentOffset))
        (:then_2
          (Timeline|WallSpawner PlayFromStart))))))

(event EventTick
  (params (DeltaSeconds :type Float%20%28single-precision%29))
  (bind _mousexspeed (Variables|Default|GetMouseXSpeed))
  (bind _player (Variables|Default|GetPlayer))
  (bind _returnvalue (* DeltaSeconds _mousexspeed))
  (bind _output_get (Variables|Default|SetCurrentMorph (Math|Vector2D|MakeVector2D (Math|Float|%(Float) (.x (+ (Variables|Default|GetCurrentMorph) (Math|Vector2D|MakeVector2D (* (Class|Actor|GetInputAxisKeyValue) _returnvalue) (* _returnvalue (Class|Actor|GetInputAxisKeyValue))))) 1.0) (Math|Float|%(Float) (.y (+ (Variables|Default|GetCurrentMorph) (Math|Vector2D|MakeVector2D (* (Class|Actor|GetInputAxisKeyValue) _returnvalue) (* _returnvalue (Class|Actor|GetInputAxisKeyValue))))) 1.0))))
  (Utilities|FlowControl|Sequence
    (:then_0
      (Components|SkeletalMesh|SetMorphTarget _player "Location" (.x (- "(X=1.000000,Y=1.000000)" (* (Math|Vector2D|MakeVector2D (Math|Float|Absolute(Float) (.x (- _output_get 0.5))) (Math|Float|Absolute(Float) (.y (- _output_get 0.5)))) 2.0))) true))
    (:then_1
      (Components|SkeletalMesh|SetMorphTarget _player "Rotation" (.y (- "(X=1.000000,Y=1.000000)" (* (Math|Vector2D|MakeVector2D (Math|Float|Absolute(Float) (.x (- _output_get 0.5))) (Math|Float|Absolute(Float) (.y (- _output_get 0.5)))) 2.0))) true))))

(fn ConstructionScript)

(fn SetCurrentOffset
  (Variables|Default|SetCurrentMorph (Math|Vector2D|MakeVector2D (Math|Random|RandomFloat) (Math|Random|RandomFloat))))