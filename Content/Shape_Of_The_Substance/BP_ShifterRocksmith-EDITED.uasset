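; Player Blueprint for a shape-matching game, where the player morphs a Substance-driven shape to match incoming walls.
; Each tick, normalized mouse position becomes the shape value, fed to the Substance graph and rendered asynchronously.
; CalculateOutcome compares wall and player values by 2D distance, driving score, combo, camera shake, feedback and health loss.
; Holding Space speeds up global time; GameOver is an unreachable stub, as health clamps at zero.
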(event Custom|CalculateOutcome
  (params (WallShapeValue :type Vector%202D%20Structure))
  (bind _gamestateref (Variables|Default|GetGameStateRef))
  ;[0 0 0] Calculate outcome with walls collided
  (bind _output_get (Variables|Default|SetShapeDifferenceCurrent (Math|Vector2D|Vector2DLength (- WallShapeValue (Variables|Default|GetCurrentPlayerShape)))))
  (if (< _output_get (Variables|Default|GetShapeDifferenceComboTolerance))
    (Default|AddScore _gamestateref (- 3.0 (Variables|Default|GetShapeDifferenceCurrent)))
    (Default|AddCombo _gamestateref)
    (Class|PlayerController|ClientPlayCameraShake (Game|GetPlayerController 0) "/Game/Shape_Of_The_Substance/CameraShake/BP_CameraShake.BP_CameraShake_C" 1.0 "CameraLocal" "4.000000, 0,3.000000")
    (Audio|Components|Audio|Play (Variables|Default|GetFeedbackPositive) 0.0)
    (else
      (Default|ResetCombo (Variables|Default|GetGameStateRef))
      (Class|PlayerController|ClientPlayCameraShake (Game|GetPlayerController 0) "/Game/Shape_Of_The_Substance/CameraShake/BP_CameraShake.BP_CameraShake_C" 3.0 "CameraLocal" "4.000000, 0,3.000000")
      (Audio|Components|Audio|Play (Variables|Default|GetFeedbackNegative) 0.0)
      (CallFunction|HealthDecrement))))

(event Custom|HealthDecrement
  ;[1 1 1] Decrement health and check for game over
  (bind _output_get (Variables|Default|SetCurrentHealth (Math|Integer|Clamp(Integer) (- (Variables|Default|GetCurrentHealth) 1) 0 (Variables|Default|GetCurrentHealth))))
  (if (< _output_get 0)
    (CallFunction|GameOver)))

(event Custom|GameOver
  (Utilities|IsValid (Variables|Default|GetGameStateRef)))

(event EventBeginPlay
  (bind _asbp_game_state (Utilities|Casting|CastToBP_GameState (Game|GetGameState)))
  (Variables|Default|SetGameStateRef _asbp_game_state)
  (Variables|Default|SetCurrentHealth (Variables|Default|GetStartingHealth)))

(event EventTick
  (params (DeltaSeconds :type Float%20%28single-precision%29))
  (bind _substance (Variables|Default|GetSubstance))
  (Utilities|FlowControl|Sequence
    (:then_0
      ;[0 0 0] Mouse Control
      (bind _returnvalue (Class|WidgetLayoutLibrary|GetMousePositiononViewport))
      (Variables|Default|SetCurrentPlayerShape (/ _returnvalue (Viewport|GetViewportSize))))
    (:then_1
      ;[0 0 0] Update Substance
      (Class|SubstanceGraphInstance|SetInputFloat _substance "Location" (Utilities|Array|MakeArray (.x (Variables|Default|GetCurrentPlayerShape)) (.y (Variables|Default|GetCurrentPlayerShape))))
      (Class|SubstanceUtility|AsyncRendering _substance))))

(event Input|KeyboardEvents|SpaceBar
  (params (Key :type Key%20Structure))
  (:Pressed
    (Utilities|Time|SetGlobalTimeDilation 2.5))
  (:Released
    (Utilities|Time|SetGlobalTimeDilation 1.0)))

(fn ConstructionScript)