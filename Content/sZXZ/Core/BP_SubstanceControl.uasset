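; BP_SubstanceControl lets the player steer a "Location" input on a Substance graph with the MoveRight and MoveForward axes.
; The axis events store their values, with the forward axis inverted, and Tick integrates them by Speed and delta time into X/Y coordinates clamped to 0–1.
; Tick pushes the coordinates to the Substance and requests asynchronous rendering every frame, as the "value changed" check is always true.
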(event EventBeginPlay)

(event EventTick
  (params (DeltaSeconds :type Float%20%28single-precision%29))
  (bind _substance (Variables|Default|GetSubstance))
  (bind _speed (Variables|Default|GetSpeed))
  ;[1 1 1] Check if value changed
  (if true
    (bind _output_get (Variables|Default|SetcurrentX (Math|Float|Clamp(Float) (+ (Variables|Default|GetcurrentX) (* (Variables|Default|GetAxisX) DeltaSeconds _speed)))))
    (bind _output_get_2 (Variables|Default|SetcurrentY (Math|Float|Clamp(Float) (+ (Variables|Default|GetcurrentY) (* (Variables|Default|GetAxisY) DeltaSeconds _speed)))))
    ;[1 1 1] Update substance
    (Class|SubstanceGraphInstance|SetInputFloat _substance "Location" (Utilities|Array|MakeArray _output_get _output_get_2))
    (Class|SubstanceUtility|AsyncRendering _substance)))

(event Collision|EventActorBeginOverlap
  (params (OtherActor :type Actor%20Object%20Reference)))

(event Input|AxisEvents|InputAxisMoveRight
  (params (AxisValue :type Float%20%28single-precision%29))
  (Variables|Default|SetAxisX AxisValue))

(event Input|AxisEvents|InputAxisMoveForward
  (params (AxisValue :type Float%20%28single-precision%29))
  (Variables|Default|SetAxisY (* AxisValue -1.0)))

(fn ConstructionScript)