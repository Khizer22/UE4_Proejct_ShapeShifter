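; BP_WallManager spawns and recycles substance-themed BP_Wall obstacles that move towards the player.
; At BeginPlay it builds a pool of walls, each with its own substance and material, then announces and waits out a start delay.
; It launches an initial batch, then a looping timer activates the first hidden wall, placing it a fixed X offset behind the last one spawned.
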(event Custom|CreateWalls
  ;[0 0 0] Create default walls and hide them to be re used later
  (for _index (range 0 8)
    (bind _returnvalue (Game|SpawnActorfromClass "/Game/Khizer/Blueprint/BP_Wall.BP_Wall_C" (Math|Transform|MakeTransform (Variables|Default|GetSpawnLocation) "90.000000,0.000000, 0" "1,1,1") "Undefined" 0 (Utilities|Array|Get(acopy) (Variables|Default|GetSubstances) _index) (Utilities|Array|Get(acopy) (Variables|Default|GetWallMaterialInstances) _index) 0))
    (Utilities|Array|Add (Variables|Default|GetWalls) _returnvalue)))

(event Custom|Spawner
  (CallFunction|SpawnAWall))

(event Custom|MoveTowardsPlayer
  (params (WallIndex :type Integer))
  (bind _walls (Variables|Default|GetWalls))
  (bind _output (Utilities|Array|Get(acopy) _walls WallIndex))
  ;[0 0 0] Move the wall towards the player
  (Transformation|SetActorLocation _output (Variables|Default|GetSpawnLocation) false false)
  (Default|BeginMovingTowardsPlayer _output))

(event Custom|InitialSpawnWalls
  ;[0.02604 0.02604 0.02604] Spawn 4 default walls when game starts
  (for _index (range 0 3)
    (CallFunction|SpawnAWall)))

(event Custom|SpawnAWall
  ;[0.004478 0.005208 0] Spawn A  Wall - 2000 units behind the last spawned wall
  (bind (_array_element _array_index) (Utilities|Array|ForEachLoopwithBreak (Variables|Default|GetWalls) :!label _label)
    (:LoopBody
      (if (Variables|/Script/Engine.Actor|GetbHidden _array_element)
        (Utilities|IsValid (Variables|Default|GetLastWallSpawned)
          (:Is%20Valid
            (Variables|Default|SetSpawnLocation (Math|Vector|MakeVector (+ (.x (Transformation|GetActorLocation (Variables|Default|GetLastWallSpawned))) 2e+03) (.y (Transformation|GetActorLocation (Variables|Default|GetLastWallSpawned))) (.z (Transformation|GetActorLocation (Variables|Default|GetLastWallSpawned))))))
          (:Is%20Not%20Valid
            _))
        (CallFunction|MoveTowardsPlayer _array_index)
        (Variables|Default|SetLastWallSpawned _array_element)
        (goto _label Break)))))

(event EventBeginPlay
  (CallFunction|CreateWalls)
  (Development|PrintString (Utilities|String|Append "Game will start in " (Utilities|String|ToString(Float) (Variables|Default|GetGameStartDelay)) " seconds") true true "(R=1.000000,G=0.649592,B=0.435094,A=1.000000)" 3.0)
  (Utilities|FlowControl|Delay (Variables|Default|GetGameStartDelay))
  (CallFunction|InitialSpawnWalls)
  (Utilities|Time|SetTimerbyEvent (delegate Custom|Spawner) 4.0 true))

(fn ConstructionScript)