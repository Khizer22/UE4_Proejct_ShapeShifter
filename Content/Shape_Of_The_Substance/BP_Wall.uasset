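; BP_Wall is an obstacle that presents a random shape for the player to be judged against.
; BeginMovingTowardsPlayer unhides it and picks a 2D shape value by difficulty (binary on Easy, continuous on Medium and Hard), which drives a Substance "Location" input rendered asynchronously.
; Tick draws debug text and, once X drops below a threshold, hides the wall and passes the shape to BP_ShifterRocksmith-EDITED's CalculateOutcome.
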(event Custom|BeginMovingTowardsPlayer
  ;[1 1 1] Un-Hide and move towards player || Set a random shape
  (Rendering|SetActorHiddenInGame false)
  (CallFunction|SetRandomShape))

(event Custom|DEBUG_Display
  ;[1 1 1] DEBUG
  (Rendering|Debug|DrawDebugString (Transformation|GetActorLocation) (Utilities|String|Append "Shape: " (Utilities|String|ToString(Vector2d) (Variables|Default|GetCurrentShape))) 0 "(R=0.437500,G=0.000000,B=0.000000,A=1.000000)"))

(event Custom|CalculateOutcome
  (bind _returnvalue (Game|Player|GetPlayerPawn 0))
  (bind (_asbp_shifter_rocksmith__edited _bsuccess) (Utilities|Casting|CastToBP_ShifterRocksmith-EDITED _returnvalue))
  ;[1 1 1] Calculate outcome on collision with player
  (if (not (Variables|Rendering|GetbHidden))
    (Rendering|SetActorHiddenInGame true)
    (if _bsuccess
      (Default|CalculateOutcome _asbp_shifter_rocksmith__edited (Variables|Default|GetCurrentShape)))))

(event Custom|SetRandomShape
  (bind _substance (Variables|Default|GetSubstance))
  (bind _substance_2 (Variables|Default|GetSubstance))
  (switch Utilities|FlowControl|Switch|SwitchonEnum_Difficulty (Variables|Default|GetDifficulty)
    (:NewEnumerator0
      ;[1 1 1] Easy
      (bind _output_get (Variables|Default|SetCurrentShape (Math|Vector2D|MakeVector2D (Math|Conversions|ToFloat(Integer) (Math|Random|RandomIntegerinRange 0 1)) (Math|Conversions|ToFloat(Integer) (Math|Random|RandomIntegerinRange 0 1)))))
      (Class|SubstanceGraphInstance|SetInputFloat _substance "Location" (Utilities|Array|MakeArray (.x _output_get) (.y _output_get)))
      (Class|SubstanceUtility|AsyncRendering _substance))
    (:NewEnumerator1
      (bind _output_get_2 (Variables|Default|SetCurrentShape (Math|Vector2D|MakeVector2D (Math|Random|RandomFloat) (Math|Random|RandomFloat)) :!label _label))
      (Class|SubstanceGraphInstance|SetInputFloat _substance_2 "Location" (Utilities|Array|MakeArray (.x _output_get_2) (.y _output_get_2)))
      (Class|SubstanceUtility|AsyncRendering _substance_2))
    (:NewEnumerator2
      (goto _label))))

(event EventBeginPlay
  (Rendering|Material|SetMaterial (Variables|Default|GetWall) 0 (Variables|Default|GetMaterialInstance)))

(event EventTick
  (params (DeltaSeconds :type Float%20%28single-precision%29))
  ;[1 1 1] debug
  (CallFunction|DEBUGDisplay)
  (if (< (.x (Transformation|GetActorLocation)) 1e+01)
    (CallFunction|CalculateOutcome)))

(fn ConstructionScript)