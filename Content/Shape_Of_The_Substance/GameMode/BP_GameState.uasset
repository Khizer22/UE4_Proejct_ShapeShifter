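; BP_GameState is the game state Blueprint that tracks score, combo and difficulty and creates the in-game UI widget on BeginPlay.
; Combo increments record the highest combo, show the combo text and periodically add health through the UI once a combo threshold is reached.
; Resetting the combo hides the text and subtracts health.
; Added score raises a difficulty enum at fixed score thresholds.
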(event Custom|AddScore
  (params (ScoreToAdd :type Float%20%28single-precision%29))
  ;[0.02083 0.007991 0.000117] Score Increment
  (bind _output_get (Variables|Default|SetScore (+ ScoreToAdd (Variables|Default|GetScore))))
  (if (> _output_get 25.0)
    (Variables|Default|SetDifficulty "NewEnumerator2")
    (elif (> _output_get 5.0)
      (Variables|Default|SetDifficulty "NewEnumerator1"))))

(event Custom|AddCombo
  ;[0.02083 0.007991 0.000117] Combo Increment
  (bind _result (Math|Integer|IncrementInt (Variables|Default|GetComboAmount))
    (:%20%20
      (Math|Integer|IncrementInt (Variables|Default|GetHealthIncreaseComboAmount)
        (:%20%20
          (if (> _result (Variables|Default|GetHighestComboAchieved))
            (Variables|Default|SetHighestComboAchieved _result))
          (Widget|SetVisibility (Variables|/Game/Shape_Of_The_Substance/Widgets/WBP_InGameUI.WBP_InGameUI_C|GetComboText (Variables|Default|GetInGameUI)) "Visible")
          (if (>= (Variables|Default|GetHealthIncreaseComboAmount) (Variables|Default|GetHealthIncreaseComboNeeded))
            (Default|AddHealth (Variables|Default|GetInGameUI))
            (Variables|Default|SetHealthIncreaseComboAmount 0)))))))

(event Custom|ResetCombo
  (bind _ingameui (Variables|Default|GetInGameUI))
  ;[0.02083 0.007991 0.000117] Reset Combo
  (Variables|Default|SetComboAmount 0)
  (Widget|SetVisibility (Variables|/Game/Shape_Of_The_Substance/Widgets/WBP_InGameUI.WBP_InGameUI_C|GetComboText _ingameui) "Hidden")
  (Default|SubtractHealth _ingameui))

(event EventBeginPlay
  ;[1 1 1] Create In Game UI
  (bind _returnvalue (UserInterface|CreateWidget "/Game/Shape_Of_The_Substance/Widgets/WBP_InGameUI.WBP_InGameUI_C" (Game|GetPlayerController 0)))
  (bind _output_get (Variables|Default|SetInGameUI _returnvalue))
  (UserInterface|Viewport|AddtoViewport _output_get 0))

(fn ConstructionScript)